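; BP_TestLootableItem is a test lootable item that shows an item card widget while hovered.
; On BeginPlay it creates a WBP_ItemCard from its item data, adds it to the viewport collapsed and sizes it to its desired size after a layout prepass.
; Hover begin makes the card visible without hit testing and updates its position, and hover end collapses it again.
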(event EventBeginPlay
  (|CallParentFunction)
  (bind _returnvalue (UserInterface|CreateWidget "/Game/Hallucinations/UI/Inventory/WBP_ItemCard.WBP_ItemCard_C" (Game|GetPlayerController 0) (Variables|/Script/Hallucinations.HInventoryItem|GetData (Variables|Default|GetItemData))))
  (bind _output_get (Variables|Default|SetItemCard _returnvalue))
  (Class|Widget|ForceLayoutPrepass _output_get)
  (UserInterface|Viewport|AddtoViewport _output_get 0)
  (Widget|SetVisibility _output_get "Collapsed")
  (Class|UserWidget|SetDesiredSizeinViewport _output_get (Class|Widget|GetDesiredSize _output_get)))

(event EventOnHoverBegin
  (bind _itemcard (Variables|Default|GetItemCard))
  (Widget|SetVisibility _itemcard "HitTestInvisible")
  (Default|UpdatePosition _itemcard))

(event EventOnHoverEnd
  (Widget|SetVisibility (Variables|Default|GetItemCard) "Collapsed"))

(fn ConstructionScript)