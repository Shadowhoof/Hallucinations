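; BP_LevelExit is a level exit that shows its level name in a tooltip while hovered.
; On BeginPlay it creates a WBP_BasicTooltip for the first player controller, sets its text from LevelName, positions it and hides it.
; Hover begin reveals the tooltip without blocking hit tests and updates its position once, and hover end hides it.
; The graph contains no travel logic.
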(event EventBeginPlay
  (bind _returnvalue (UserInterface|CreateWidget "/Game/Hallucinations/UI/Common/WBP_BasicTooltip.WBP_BasicTooltip_C" (Game|GetPlayerController 0)))
  (UserInterface|Viewport|AddtoViewport _returnvalue 0)
  (bind _output_get (Variables|Default|SetTooltipWidget _returnvalue))
  (Default|SetText _output_get (Utilities|Text|ToText(Name) (Variables|Default|GetLevelName)))
  (Default|UpdatePosition _output_get)
  (Widget|SetVisibility _output_get "Hidden"))

(event EventOnHoverEnd
  (Widget|SetVisibility (Variables|Default|GetTooltipWidget) "Hidden"))

(event EventOnHoverBegin
  (bind _tooltipwidget (Variables|Default|GetTooltipWidget))
  (Widget|SetVisibility _tooltipwidget "SelfHitTestInvisible")
  (Default|UpdatePosition _tooltipwidget))

(fn ConstructionScript)