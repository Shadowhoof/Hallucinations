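; Player controller that manages the player's on-screen UI for the HUD and death screen.
; BeginPlay creates the HUD widget and adds it to the viewport.
; OnPawnDeath creates a death screen widget, stores it and displays it, and OnPlayerRestart removes that stored widget if it is still valid.
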(event EventBeginPlay
  (bind _returnvalue (UserInterface|CreateWidget "/Game/Hallucinations/UI/WBP_HUD.WBP_HUD_C" self))
  (UserInterface|Viewport|AddtoViewport _returnvalue 0))

(event EventOnPlayerRestart
  (bind _deathwidget (Variables|Default|GetDeathWidget))
  (Utilities|IsValid _deathwidget
    (:Is%20Valid
      (Widget|RemovefromParent _deathwidget))))

(event EventOnPawnDeath
  (params (Killer :type H%20Character%20Object%20Reference) (Victim :type Actor%20Object%20Reference))
  (bind _returnvalue (UserInterface|CreateWidget "/Game/Hallucinations/UI/WBP_DeathScreen.WBP_DeathScreen_C" self))
  (bind _output_get (Variables|Default|SetDeathWidget _returnvalue))
  (UserInterface|Viewport|AddtoViewport _output_get 0))

(fn ConstructionScript)