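; Player character Blueprint that owns the HUD widgets for the action bar, skill book, inventory and equipment.
; BeginPlay creates the action bar and a collapsed skill book from the character's components, then subscribes to inventory changes to refresh the inventory widget.
; Toggle events flip widget visibility, refreshing inventory and equipment when shown, and helper functions expose the action bar lock.
; Tick prints every AttributeSet value on screen as a debug readout.
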(event EventBeginPlay
  (bind _returnvalue (Pawn|GetController))
  (bind _abilitycomponent (Variables|Default|GetAbilityComponent))
  (bind _asplayer_controller (Utilities|Casting|CastToPlayerController _returnvalue))
  ;[1 1 1] Create Action Bar widget
  (bind _returnvalue_2 (UserInterface|CreateWidget "/Game/Hallucinations/UI/Abilities/WBP_ActionBar.WBP_ActionBar_C" _asplayer_controller (Variables|Default|GetActionBarComponent) _abilitycomponent))
  (bind _output_get (Variables|Default|SetActionBarWidget _returnvalue_2))
  (UserInterface|Viewport|AddtoViewport _output_get 0)
  ;[1 1 1] Create Skill Book Widget
  (bind _returnvalue_3 (UserInterface|CreateWidget "/Game/Hallucinations/UI/Abilities/WBP_SkillBook.WBP_SkillBook_C" _asplayer_controller _abilitycomponent))
  (bind _output_get_2 (Variables|Default|SetSkillBookWidget _returnvalue_3))
  (UserInterface|Viewport|AddtoViewport _output_get_2 0)
  (Widget|SetVisibility _output_get_2 "Collapsed")
  ;[1 1 1] Subscribe to Inventory Event
  (EventDispatchers|BindEventtoOnInventoryChanged (Variables|Default|GetInventoryComponent) (EventDispatchers|CreateEvent :!event OnInventoryUpdated)))

(event EventToggleSkillBook
  (UI|ToggleWidgetVisibility (Variables|Default|GetSkillBookWidget)))

(event EventTick
  (params (DeltaSeconds :type Float%20%28single-precision%29))
  (bind _attributecomponent (Variables|Default|GetAttributeComponent))
  (bind _attributeset (Variables|/Script/Hallucinations.HAttributeComponent|GetAttributeSet _attributecomponent))
  (bind _attributes (Variables|/Script/Hallucinations.AttributeSet|GetAttributes _attributeset))
  (bind _keys (Utilities|Map|Keys _attributes))
  (for _array_element _keys
    (Development|PrintString (Utilities|String|ToString(Text) (Utilities|Text|FormatText "{Attribute} : {Value}" (Utilities|String|EnumtoString _array_element) (.CurrentValue (Utilities|Struct|BreakAttributeData (.Value (Utilities|Map|Find _attributes _array_element)))))) true false "(R=0.838666,G=0.130349,B=1.000000,A=1.000000)" 0.0)))

(event EventToggleInventory
  (bind _inventorywidget (Variables|Default|GetInventoryWidget))
  (UI|ToggleWidgetVisibility (Variables|Default|GetEquipmentWidget))
  (bind _is_visible (UI|ToggleWidgetVisibility _inventorywidget))
  (if _is_visible
    (Default|UpdateInventory _inventorywidget)
    (Default|RefreshEquipment (Variables|Default|GetEquipmentWidget))))

(fn ConstructionScript)

(fn SetActionBarLock
  (params (IsLocked :type Boolean))
  (Variables|/Game/Hallucinations/UI/Abilities/WBP_ActionBar.WBP_ActionBar_C|SetIsLocked (Variables|Default|GetActionBarWidget) IsLocked))

(fn IsActionBarLocked
  (return (Variables|/Game/Hallucinations/UI/Abilities/WBP_ActionBar.WBP_ActionBar_C|GetIsLocked (Variables|Default|GetActionBarWidget))))

(fn ToggleWidgetVisibility
  (params (Widget :type User%20Widget%20Object%20Reference))
  (bind _returnvalue (Widget|IsVisible Widget))
  (if _returnvalue
    (Widget|SetVisibility Widget "Collapsed")
    (else
      (Widget|SetVisibility Widget "SelfHitTestInvisible")))
  (return _returnvalue))

(fn OnInventoryUpdated
  (params (InventoryComponent :type H%20Inventory%20Component%20Object%20Reference))
  (Default|UpdateInventory (Variables|Default|GetInventoryWidget)))